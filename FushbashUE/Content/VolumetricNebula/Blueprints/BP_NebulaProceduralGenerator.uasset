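; Procedural nebula actor that scatters raymarched volumetric sphere meshes on a flat disc, built in the construction script from a seeded random stream.
; Random placements are rejected by sphere overlap tests against temporary collision spheres, with capped attempts, and those spheres are destroyed afterwards.
; Each mesh gets a dynamic instance of a random material with randomized color, density and four internal lights.
; A quality tier sets raymarch settings, distance textures and compensating multipliers.
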(event `self.ReceiveBeginPlay`)

(fn `CreateMaterialInstance`
  (returns (Material :type "MaterialInstanceDynamic Object Reference"))
  (locals (MaterialInstance :type "MaterialInstanceDynamic Object Reference") (DensityMultiplier :type "Float (double-precision)" :default 1.0) (FogMultiplier :type "Float (double-precision)") (MaterialIndex :type Integer))
  (bind _output_get (set `local.MaterialIndex` (`.OutIndex` (`KismetArrayLibrary.Array_RandomFromStream` (`self.Materials`) (`self.RandomStream`)))))
  (bind _returnvalue (`KismetMaterialLibrary.CreateDynamicMaterialInstance` (`|GetArrayItem` (`self.Materials`) _output_get)))
  (set `local.MaterialInstance` _returnvalue)
  (`|ExecutionSequence`
    (:`then_0`
      ;[1 1 1] Set quality material parameters
      (switch `/Game/VolumetricNebula/Blueprints/Quality` (`self.Quality`)
        (:`NewEnumerator0`
          (`MaterialInstanceDynamic.SetScalarParameterValue` (`local.MaterialInstance`) "Raymarching Steps" 250.0)
          (`MaterialInstanceDynamic.SetScalarParameterValue` (`local.MaterialInstance`) "Start Step Size" 15.0)
          (`MaterialInstanceDynamic.SetScalarParameterValue` (`local.MaterialInstance`) "Step Size Multiplier" 0.0015)
          (`MaterialInstanceDynamic.SetScalarParameterValue` (`local.MaterialInstance`) "Distance Bias" 130.0)
          (`MaterialInstanceDynamic.SetTextureParameterValue` (`local.MaterialInstance`) "Distance Texture" (`|GetArrayItem` (`self.DistanceTexturesLow`) (`local.MaterialIndex`)))
          (set `local.DensityMultiplier` 2.0)
          (set `local.FogMultiplier` 2.4))
        (:`NewEnumerator1`
          (`MaterialInstanceDynamic.SetScalarParameterValue` (`local.MaterialInstance`) "Raymarching Steps" 300.0)
          (`MaterialInstanceDynamic.SetScalarParameterValue` (`local.MaterialInstance`) "Start Step Size" 12.0)
          (`MaterialInstanceDynamic.SetScalarParameterValue` (`local.MaterialInstance`) "Step Size Multiplier" 0.0012)
          (`MaterialInstanceDynamic.SetScalarParameterValue` (`local.MaterialInstance`) "Distance Bias" 110.0)
          (`MaterialInstanceDynamic.SetTextureParameterValue` (`local.MaterialInstance`) "Distance Texture" (`|GetArrayItem` (`self.DistanceTexturesMedium`) (`local.MaterialIndex`)))
          (set `local.DensityMultiplier` 1.7)
          (set `local.FogMultiplier` 1.8))
        (:`NewEnumerator2`
          (`MaterialInstanceDynamic.SetScalarParameterValue` (`local.MaterialInstance`) "Raymarching Steps" 350.0)
          (`MaterialInstanceDynamic.SetScalarParameterValue` (`local.MaterialInstance`) "Start Step Size" 10.0)
          (`MaterialInstanceDynamic.SetScalarParameterValue` (`local.MaterialInstance`) "Step Size Multiplier" 0.001)
          (`MaterialInstanceDynamic.SetScalarParameterValue` (`local.MaterialInstance`) "Distance Bias" 90.0)
          (`MaterialInstanceDynamic.SetTextureParameterValue` (`local.MaterialInstance`) "Distance Texture" (`|GetArrayItem` (`self.DistanceTexturesHigh`) (`local.MaterialIndex`)))
          (set `local.DensityMultiplier` 1.4)
          (set `local.FogMultiplier` 1.4))
        (:`NewEnumerator3`
          (`MaterialInstanceDynamic.SetScalarParameterValue` (`local.MaterialInstance`) "Raymarching Steps" 400.0)
          (`MaterialInstanceDynamic.SetScalarParameterValue` (`local.MaterialInstance`) "Start Step Size" 7.0)
          (`MaterialInstanceDynamic.SetScalarParameterValue` (`local.MaterialInstance`) "Step Size Multiplier" 0.0007)
          (`MaterialInstanceDynamic.SetScalarParameterValue` (`local.MaterialInstance`) "Distance Bias" 80.0)
          (`MaterialInstanceDynamic.SetTextureParameterValue` (`local.MaterialInstance`) "Distance Texture" (`|GetArrayItem` (`self.DistanceTexturesUltra`) (`local.MaterialIndex`)))
          (set `local.DensityMultiplier` 1.0)
          (set `local.FogMultiplier` 1.0))))
    (:`then_1`
      ;[1 1 1] Set nebula density material parameters
      (`MaterialInstanceDynamic.SetVectorParameterValue` (`local.MaterialInstance`) "Nebula Color" (* (`KismetMathLibrary.LinearColorLerp` (`self.Nebula Color 1`) (`self.Nebula Color 2`) (`KismetMathLibrary.RandomFloatFromStream` (`self.RandomStream`))) (* (`KismetMathLibrary.RandomFloatInRangeFromStream` (`self.Min Nebula Emission`) (`self.Max Nebula Emission`) (`self.RandomStream`)) 0.01)))
      (`MaterialInstanceDynamic.SetScalarParameterValue` (`local.MaterialInstance`) "Fog Density" (* (* (`self.Fog Density`) 0.0001) (`local.FogMultiplier`)))
      (`MaterialInstanceDynamic.SetScalarParameterValue` (`local.MaterialInstance`) "Nebula Density" (* (* (`KismetMathLibrary.RandomFloatInRangeFromStream` (`self.Min Nebula Density`) (`self.Max Nebula Density`) (`self.RandomStream`)) 1000000.0) (`local.DensityMultiplier`)))
      (`MaterialInstanceDynamic.SetScalarParameterValue` (`local.MaterialInstance`) "Fade In Radius" (`self.Fade In Radius`)))
    (:`then_2`
      ;[1 1 1] Set post processing material parameters
      (`MaterialInstanceDynamic.SetScalarParameterValue` (`local.MaterialInstance`) "Brightness" (`self.Brightness`))
      (`MaterialInstanceDynamic.SetScalarParameterValue` (`local.MaterialInstance`) "Opacity" (`self.Opacity`))
      (`MaterialInstanceDynamic.SetScalarParameterValue` (`local.MaterialInstance`) "Contrast" (`self.Contrast`))
      (`MaterialInstanceDynamic.SetScalarParameterValue` (`local.MaterialInstance`) "Saturation" (`self.Saturation`))
      (`MaterialInstanceDynamic.SetScalarParameterValue` (`local.MaterialInstance`) "Power" (`self.Power`))
      (`MaterialInstanceDynamic.SetVectorParameterValue` (`local.MaterialInstance`) "Tint" (`self.Tint`)))
    (:`then_3`
      (`self.SetLightMaterialParameters` (`local.MaterialInstance`)))
    (:`then_4`
      (return (`local.MaterialInstance`)))))

(fn `GenerateNebula`
  (locals (SpawnedSphereAmount :type Integer) (Iteration :type Integer))
  (set `self.RandomStream` (`KismetMathLibrary.MakeRandomStream` (`self.Random Seed`)))
  (while (and (< (`local.SpawnedSphereAmount`) (`self.Volumetric Sphere Amount`)) (< (`local.Iteration`) (* (`self.Volumetric Sphere Amount`) 50)))
    (`/Engine/EditorBlueprintResources/StandardMacros.IncrementInt` (`local.Iteration`)
      (:`  `
        (bind _success (`self.SpawnNebulaSphere`))
        (if _success
          (`/Engine/EditorBlueprintResources/StandardMacros.IncrementInt` (`local.SpawnedSphereAmount`))))))
  ;[1 1 1] Destroy sphere collision components after generation
  (for _array_element (`self.CollisionSpheres`)
    (`ActorComponent.K2_DestroyComponent` _array_element)))

(fn `SetLightMaterialParameters`
  (params (MaterialInstance :type "MaterialInstanceDynamic Object Reference"))
  (locals (LightMultiplier :type "Float (double-precision)" :default 1.0))
  (bind _randomstream (`self.RandomStream`))
  (for _index (range 1 5)
    (`|ExecutionSequence`
      (:`then_0`
        ;[1 1 1] Set light position material parameter
        (`MaterialInstanceDynamic.SetVectorParameterValue` (`local.MaterialInstance`) (`KismetStringLibrary.Conv_StringToName` (`KismetStringLibrary.Concat_StrStr` "Light Position " (`KismetStringLibrary.Conv_IntToString` _index))) (`KismetMathLibrary.Conv_VectorToLinearColor` (* (`KismetMathLibrary.RandomUnitVectorFromStream` _randomstream) (`KismetMathLibrary.RandomFloatInRangeFromStream` 0.0 (* (`self.SphereRadius`) 0.7) _randomstream)))))
      (:`then_1`
        ;[1 1 1] Set light color material parameter
        (switch `/Game/VolumetricNebula/Blueprints/Quality` (`self.Quality`)
          (:`NewEnumerator0`
            (set `local.LightMultiplier` 2.0))
          (:`NewEnumerator1`
            (set `local.LightMultiplier` 1.7))
          (:`NewEnumerator2`
            (set `local.LightMultiplier` 1.4))
          (:`NewEnumerator3`
            (set `local.LightMultiplier` 1.0)))
        (`MaterialInstanceDynamic.SetVectorParameterValue` (`local.MaterialInstance`) (`KismetStringLibrary.Conv_StringToName` (`KismetStringLibrary.Concat_StrStr` "Light Color " (`KismetStringLibrary.Conv_IntToString` _index))) (/ (struct :`R` 1.0 :`G` 1.0 :`B` 1.0 :`A` 1.0) (* (`KismetMathLibrary.LinearColorLerp` (`self.Light Color 1`) (`self.Light Color 2`) (`KismetMathLibrary.RandomFloatFromStream` (`self.RandomStream`))) (* (* (`KismetMathLibrary.RandomFloatInRangeFromStream` (`self.Min Light Intensity`) (`self.Max Light Intensity`) (`self.RandomStream`)) (`local.LightMultiplier`)) 0.01)))))))
  (`MaterialInstanceDynamic.SetScalarParameterValue` (`local.MaterialInstance`) "Light Intensity Limit" (* (`self.Max Light Intensity`) 5.0)))

(fn `SpawnNebulaSphere`
  (returns (Success :type Boolean))
  (locals (SphereTransform :type "Transform Structure") (ObjectTypes :type "Array of EObjectTypeQuery Enum"))
  (bind _returnvalue_x (`KismetMathLibrary.BreakVector` (`self.GetActorScale3D`)))
  (bind _randomstream (`self.RandomStream`))
  (bind (_spheretransform_location _spheretransform_rotation _spheretransform_scale) (`KismetMathLibrary.BreakTransform` (`local.SphereTransform`)))
  (bind (_returnvalue_x_2 _returnvalue_y) (`KismetMathLibrary.BreakVector` (`KismetMathLibrary.RandomUnitVectorFromStream` _randomstream)))
  ;[1 1 1] Random sphere transform
  (bind _output_get (set `local.SphereTransform` (`KismetMathLibrary.MakeTransform` (* (`KismetMathLibrary.Normal` (`KismetMathLibrary.MakeVector` _returnvalue_x_2 _returnvalue_y)) (`KismetMathLibrary.RandomFloatInRangeFromStream` 0.0 (* (`self.Nebula Radius (km)`) 100000.0) _randomstream)) (`KismetMathLibrary.RandomRotatorFromStream` true _randomstream) (`KismetMathLibrary.Conv_DoubleToVector` (/ (`KismetMathLibrary.RandomFloatInRangeFromStream` (`self.Min Sphere Radius (km)`) (`self.Max Sphere Radius (km)`) _randomstream) (* (`self.SphereRadius`) 1e-05))))))
  ;[1 1 1] Test overlap with other nebula spheres
  (bind (_outcomponents _returnvalue) (`KismetSystemLibrary.SphereOverlapComponents` (`KismetMathLibrary.TransformLocation` (`self.GetTransform`) (.location _output_get)) (* (.z (.scale _output_get)) (`self.Dispersion`) (`self.SphereRadius`) _returnvalue_x) (`local.ObjectTypes`) "/Script/Engine.SphereComponent"))
  (if _returnvalue
    (return false)
    (else
      ;[1 1 1] Add sphere collision component for overlap test
      (bind _returnvalue_2 (`AddComponent|NODE_AddSphereComponent-1` :`RelativeTransform` (`KismetMathLibrary.MakeTransform` _spheretransform_location (struct) (* _spheretransform_scale (* (`self.Dispersion`) (`self.SphereRadius`))))))
      (`KismetArrayLibrary.Array_Add` (`self.CollisionSpheres`) _returnvalue_2)
      ;[1 1 1] Spawn nebula sphere and assign dynamic material instance
      (bind _returnvalue_3 (`AddComponent|NODE_AddStaticMeshComponent-3` :`RelativeTransform` (`local.SphereTransform`)))
      (bind _material (`self.CreateMaterialInstance`))
      (`PrimitiveComponent.SetMaterial` _returnvalue_3 0 _material)
      (return true))))

(fn `UserConstructionScript`
  (`self.GenerateNebula`))